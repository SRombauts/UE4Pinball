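; BP_Ball is a physics-driven ball actor that rolls on a table under simulated gravity of arbitrary orientation.
; Each Tick applies a DefaultSpeed velocity-change impulse scaled by delta time to act as that gravity.
; It also line-traces straight down and pushes along the hit normal, scaled by TableStickyness, to keep the ball on the table.
; The trace leaves persistent debug lines.
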(event EventTick
  (params (DeltaSeconds :type Float%20%28single-precision%29))
  (bind _returnvalue (Transformation|GetActorLocation))
  ;[1 1 1] simulate arbitraty gravity orientation
  (Physics|AddImpulse (Variables|Default|GetBall) (* (Variables|Default|GetDefaultSpeed) DeltaSeconds) "None" true)
  ;[1 1 1] Stick to the table
  (bind _outhit (Collision|LineTraceByChannel _returnvalue (- _returnvalue "0, 0,500.000000") "TraceTypeQuery1" false 0 "Persistent"))
  (Physics|AddImpulse (Variables|Default|GetBall) (* (.ImpactNormal (Collision|BreakHitResult _outhit)) (* (Variables|Default|GetTableStickyness) DeltaSeconds)) "None" true))

(fn ConstructionScript)